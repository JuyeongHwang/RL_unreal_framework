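; BP_Env is a reinforcement-learning environment for a cart-pole task where the cart also seeks a goal.
; Each Tick it either streams state through BP_Network as slash-delimited messages or, once an action is flagged, applies it as cart velocity.
; It then rewards survival, penalizes goal distance and sends back observation, reward and done.
; Pole failure or timeout ends the episode, resetting the cart and randomizing the goal's X position.
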(event `self.ReceiveBeginPlay`
  ;[1 1 1] reset()
  (`self.Reset`)
  (`/Game/Blueprints/BP_cart.Init` (`self.cart`)))

(event `self.ReceiveTick`
  (params (DeltaSeconds :type "Float (single-precision)"))
  (bind _cart (`self.cart`))
  (bind _cart_2 (`self.cart`))
  (bind _cart_3 (`self.cart`))
  (bind (_returnvalue_x _returnvalue_y) (`KismetMathLibrary.BreakVector` (`self.K2_GetActorLocation` (`self.cart`))))
  (bind _cartlocation_x (`KismetMathLibrary.BreakVector` (`/Game/Blueprints/BP_cart.cartLocation` _cart)))
  (bind _polevelocity_x (`KismetMathLibrary.BreakVector` (`/Game/Blueprints/BP_cart.poleVelocity` _cart)))
  (bind _cartlocation_x_2 (`KismetMathLibrary.BreakVector` (`/Game/Blueprints/BP_cart.cartLocation` _cart_2)))
  (bind _poleangle (`/Game/Blueprints/BP_cart.poleAngle` _cart_3))
  (bind _returnvalue_x_2 (`KismetMathLibrary.BreakVector` (`SceneComponent.GetComponentVelocity` (`/Game/Blueprints/BP_cart.cart` _cart_2))))
  (bind _returnvalue_x_3 (`KismetMathLibrary.BreakVector` (`SceneComponent.GetComponentVelocity` (`/Game/Blueprints/BP_cart.cart` _cart))))
  (bind _returnvalue_x_4 (`KismetMathLibrary.BreakVector` (`PrimitiveComponent.GetPhysicsAngularVelocityInDegrees` (`/Game/Blueprints/BP_cart.pole` _cart_2) "None")))
  (bind (_returnvalue_x_5 _returnvalue_y_2) (`KismetMathLibrary.BreakVector` (`SceneComponent.K2_GetComponentLocation` (`/Game/Blueprints/BP_cart.cart` _cart_3))))
  (bind (_returnvalue_x_6 _returnvalue_y_3) (`KismetMathLibrary.BreakVector` (`SceneComponent.K2_GetComponentLocation` (`/Game/Blueprints/BP_cart.pole` _cart_3))))
  (set `self.time` (+ (`self.time`) 1))
  (if (not (`self.boolGetAction`))
    (if (`KismetArrayLibrary.Array_IsEmpty` (`self.state`))
      ;[1 1 1] state
      (`self.SetState` _cartlocation_x _returnvalue_x_3 (`/Game/Blueprints/BP_cart.poleAngle` _cart) _polevelocity_x)
      ;[1 1 1] send state data for selecting action
      (`TcpSocketConnection.SendData` (`self.Network`) 0 (`TcpSocketConnection.Conv_StringToBytes` "state/"))
      (for _array_element (`self.state`)
        (`TcpSocketConnection.SendData` (`self.Network`) 0 (`TcpSocketConnection.Conv_StringToBytes` (`KismetStringLibrary.Conv_DoubleToString` _array_element)))
        (`TcpSocketConnection.SendData` (`self.Network`) 0 (`TcpSocketConnection.Conv_StringToBytes` "/")))
      (`TcpSocketConnection.SendData` (`self.Network`) 0 (`TcpSocketConnection.Conv_StringToBytes` "stateend/")))
    (else
      ;[1 1 1] step() / 받은 action이 있으면, 행동하기.
      (`PrimitiveComponent.SetPhysicsLinearVelocity` (`/Game/Blueprints/BP_cart.cart` (`self.cart`)) (* (`KismetMathLibrary.Vector_Forward`) (`self.receivedAction`)) false "None")
      (set `self.boolGetAction` false)
      (`KismetArrayLibrary.Array_Clear` (`self.state`))
      ;[1 1 1] step()/ reward
      (set `self.reward` (+ (`self.reward`) 0.1))
      (set `self.reward` (- (`self.reward`) (* (`KismetMathLibrary.Abs` (`KismetMathLibrary.VSize` (- (`SceneComponent.K2_GetComponentLocation` (`/Game/Blueprints/BP_cart.cart` (`self.cart`))) (`self.K2_GetActorLocation` (`self.goal`))))) 1.5)))
      (set `self.episode_reward` (+ (`self.reward`) (`self.episode_reward`)))
      ;[1 1 1] step() / out condition
      (`/Game/Blueprints/BP_cart.SetPoleAngle` _cart_3)
      (if (and (<= _poleangle -0.65) (>= _poleangle -0.95))
        (set `self.reward` (- (`self.reward`) 1.0))
        (set `self.done` true :!label _label)
        (set `self.episodeCount` (+ (`self.episodeCount`) 1))
        (`KismetSystemLibrary.PrintString` "episode")
        (`KismetSystemLibrary.PrintString` (`KismetStringLibrary.Conv_IntToString` (`self.episodeCount`)))
        (`KismetSystemLibrary.PrintString` (`KismetStringLibrary.Conv_DoubleToString` (`self.episode_reward`)))
        (set `self.episode_reward` 0.0)
        (elif (>= (+ (`KismetMathLibrary.Abs` (- _returnvalue_x_5 _returnvalue_x_6)) (`KismetMathLibrary.Abs` (- _returnvalue_y_2 _returnvalue_y_3))) 20.0)
          (set `self.reward` (- (`self.reward`) 1.0))
          (goto _label)
          (elif (>= (`self.time`) 300)
            (goto _label)
            (else
              _))))
      ;[1 1 1] next state, reward, done (true : 1.0, false : 0.0)
      (`self.SetObservation` _cartlocation_x_2 _returnvalue_x_2 (`/Game/Blueprints/BP_cart.poleAngle` _cart_2) _returnvalue_x_4 (`self.reward`) (`KismetMathLibrary.Conv_BoolToDouble` (`self.done`)))
      ;[1 1 1] send state data for selecting action
      (`TcpSocketConnection.SendData` (`self.Network`) 0 (`TcpSocketConnection.Conv_StringToBytes` "obs/"))
      (for _array_element_2 (`self.observation`)
        (`TcpSocketConnection.SendData` (`self.Network`) 0 (`TcpSocketConnection.Conv_StringToBytes` (`KismetStringLibrary.Conv_DoubleToString` _array_element_2)))
        (`TcpSocketConnection.SendData` (`self.Network`) 0 (`TcpSocketConnection.Conv_StringToBytes` "/")))
      (`TcpSocketConnection.SendData` (`self.Network`) 0 (`TcpSocketConnection.Conv_StringToBytes` "obsend/"))
      (set `self.reward` 0.0)
      (`KismetArrayLibrary.Array_Clear` (`self.observation`))
      (if (`self.done`)
        (`/Game/Blueprints/BP_cart.Reset` (`self.cart`))
        (set `self.done` false)
        (set `self.time` 0)
        (set `self.episodeCount` (+ (`self.episodeCount`) 1))
        (`self.K2_SetActorLocation` (`self.goal`) (`KismetMathLibrary.MakeVector` (`KismetMathLibrary.RandomFloatInRange` -400.0 400.0) _returnvalue_y 50.0) false false)))))

(fn `Reset`
  (set `self.time` 0)
  (set `self.episode_reward` 0.0)
  (`KismetArrayLibrary.Array_Clear` (`self.state`))
  (set `self.receivedAction` 0.0)
  (bind _outactors (`GameplayStatics.GetAllActorsOfClass` "/Game/Blueprints/BP_Network.BP_Network_C"))
  (set `self.Network` (`|GetArrayItem` _outactors (`self.index`)))
  (bind _outactors_2 (`GameplayStatics.GetAllActorsOfClass` "/Game/Blueprints/BP_cart.BP_cart_C"))
  (set `self.cart` (`|GetArrayItem` _outactors_2 (`self.index`)))
  (bind _outactors_3 (`GameplayStatics.GetAllActorsOfClass` "/Game/Blueprints/BP_Goal.BP_Goal_C"))
  (set `self.goal` (`|GetArrayItem` _outactors_3 (`self.index`))))

(fn `SetObservation`
  (params (NewCartPosX :type "Float (double-precision)") (NewCartVelX :type "Float (double-precision)") (NewpoleAngle :type "Float (double-precision)") (NewpoleVelocityX :type "Float (double-precision)") (reward :type "Float (double-precision)") (done :type "Float (double-precision)"))
  (bind _observation (`self.observation`))
  (`KismetArrayLibrary.Array_Add` _observation NewCartPosX)
  (`KismetArrayLibrary.Array_Add` _observation NewCartVelX)
  (`KismetArrayLibrary.Array_Add` _observation NewpoleAngle)
  (`KismetArrayLibrary.Array_Add` _observation NewpoleVelocityX)
  (`KismetArrayLibrary.Array_Add` _observation reward)
  (`KismetArrayLibrary.Array_Add` _observation done))

(fn `SetState`
  (params (cartPositionX :type "Float (double-precision)") (cartVelX :type "Float (double-precision)") (poleAngle :type "Float (double-precision)") (poleVelocityX :type "Float (double-precision)"))
  (bind _state (`self.state`))
  (`KismetArrayLibrary.Array_Add` _state cartPositionX)
  (`KismetArrayLibrary.Array_Add` _state cartVelX)
  (`KismetArrayLibrary.Array_Add` _state poleAngle)
  (`KismetArrayLibrary.Array_Add` _state poleVelocityX))

(fn `UserConstructionScript`)