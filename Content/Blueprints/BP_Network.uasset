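; BP_Network is an actor that bridges BP_Env to an external process over a local socket connection, exchanging states and actions.
; On BeginPlay it finds BP_Env, connects to localhost and sends a greeting once connected.
; Incoming messages become BP_Env's numeric action when no state is pending.
; Tick polls BP_Env's flag and streams ready states as slash-delimited text ending in "end", then clears them.
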(event `self.ReceiveBeginPlay`
  (bind _returnvalue (`GameplayStatics.GetActorOfClass` "/Game/Blueprints/BP_Env.BP_Env_C"))
  (set `self.env` _returnvalue)
  (bind _connectionid (`self.Connect` "127.0.0.1" 5052 (delegate `disconnected`) (delegate `connected`) (delegate `message_recd`)))
  (set `self.ConID` _connectionid))

(event `disconnected`
  (params (ConnectionId :type Integer)))

(event `connected`
  (params (ConnectionId :type Integer))
  (`KismetSystemLibrary.PrintString` "Connect...")
  (`self.SendData` 0 (`self.Conv_StringToBytes` "I'm Unreal."))
  (`KismetSystemLibrary.PrintString` "Compltet Networkl."))

(event `message_recd`
  (params (ConnectionId :type Integer) (Message :type "Array of Byte (by ref)"))
  (bind _env (`self.env`))
  (bind _env_2 (`self.env`))
  (bind _returnvalue (`self.Message_ReadString` Message (`KismetArrayLibrary.Array_Length` Message)))
  (if (`/Game/Blueprints/BP_Env.boolState` _env)
    (`KismetSystemLibrary.PrintString` "else")
    (elif (`KismetArrayLibrary.Array_IsEmpty` (`/Game/Blueprints/BP_Env.state` _env))
      (`KismetSystemLibrary.PrintString` "action")
      (bind _output_get (set `/Game/Blueprints/BP_Env.receivedAction` (`KismetStringLibrary.Conv_StringToDouble` _returnvalue) _env_2))
      (set `/Game/Blueprints/BP_Env.boolAction` true _env_2)
      (`KismetSystemLibrary.PrintString` (`KismetStringLibrary.Conv_DoubleToString` _output_get)))))

(event `self.ReceiveTick`
  (params (DeltaSeconds :type "Float (single-precision)"))
  (bind _env (`self.env`))
  ;[1 1 1] Send State
  (if (and (`/Game/Blueprints/BP_Env.boolState` _env) (`KismetArrayLibrary.Array_IsNotEmpty` (`/Game/Blueprints/BP_Env.state` _env)))
    (`KismetSystemLibrary.PrintString` "Send state")
    (`|ExecutionSequence`
      (:`then_0`
        (`self.SendData` 0 (`self.Conv_StringToBytes` "state/")))
      (:`then_1`
        (for _array_element (`/Game/Blueprints/BP_Env.state` (`self.env`))
          (`self.SendData` 0 (`self.Conv_StringToBytes` (`KismetStringLibrary.Conv_DoubleToString` _array_element)))
          (`self.SendData` 0 (`self.Conv_StringToBytes` "/")))
        (set `/Game/Blueprints/BP_Env.boolState` false (`self.env`))
        (`self.SendData` 0 (`self.Conv_StringToBytes` "end"))
        (`KismetArrayLibrary.Array_Clear` (`/Game/Blueprints/BP_Env.state` (`self.env`)))))))

(fn `UserConstructionScript`)