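; Cart-pole actor, apparently for reinforcement learning, with a Cart and Pole that expose state through callable functions.
; Init caches start transforms and finds BP_Env; Reset teleports both parts back and zeroes stored variables, not physics velocities.
; SetPoleAngle stores the pole-to-floor cosine as PoleAngle, mixing relative and world positions; CollectObservations appends samples to arrays.
; EventGraph's movement, reward and termination logic is disconnected and never runs.
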(event `self.ReceiveBeginPlay`)

(event `self.ReceiveTick`
  (params (DeltaSeconds :type "Float (single-precision)")))

(fn `CollectObservations`
  (params (cartPosition :type "Vector Structure") (cartVelocity :type "Vector Structure") (poleVelocity :type "Vector Structure") (poleAngle :type "Float (double-precision)"))
  (locals (localPositions :type "Array of Vector Structure") (velocities :type "Array of Vector Structure") (angularVelocity :type "Array of Vector Structure") (poleAngles :type "Array of Float (double-precision)"))
  (`KismetArrayLibrary.Array_Add` (`local.localPositions`) cartPosition)
  (`KismetArrayLibrary.Array_Add` (`local.velocities`) cartVelocity)
  (`KismetArrayLibrary.Array_Add` (`local.angularVelocity`) poleVelocity)
  (`KismetArrayLibrary.Array_Add` (`local.poleAngles`) poleAngle))

(fn `Init`
  (set `self.OriginCubeTransform` (`SceneComponent.K2_GetComponentToWorld` (`self.cart`)))
  (set `self.OriginCylinderTransform` (`SceneComponent.K2_GetComponentToWorld` (`self.pole`)))
  (bind _returnvalue (`GameplayStatics.GetActorOfClass` "/Game/Blueprints/BP_Env.BP_Env_C"))
  (set `self.env` _returnvalue)
  (set `self.poleAngle` 0.0)
  (set `self.poleVelocity` (0.0 0.0 0.0))
  (set `self.cartVelocity` (0.0 0.0 0.0))
  (set `self.cartLocation` (.location (`self.OriginCubeTransform`))))

(fn `Reset`
  (`SceneComponent.K2_SetWorldTransform` (`self.cart`) (`self.OriginCubeTransform`) false true)
  (`SceneComponent.K2_SetWorldTransform` (`self.pole`) (`self.OriginCylinderTransform`) false true)
  (set `self.poleVelocity` (0.0 0.0 0.0))
  (set `self.cartVelocity` (0.0 0.0 0.0))
  (set `self.poleAngle` 0.0))

(fn `SetPoleAngle`
  (locals (Aprime :type "Vector Structure"))
  (bind (_returnvalue_x _returnvalue_y _returnvalue_z) (`KismetMathLibrary.BreakVector` (`SceneComponent.K2_GetComponentLocation` (`self.pole`))))
  (bind (_relativelocation_x _relativelocation_y) (`KismetMathLibrary.BreakVector` (`SceneComponent.RelativeLocation` (`self.pole_end`))))
  ;[1 1 1] 막대기 각도 & 지면 각도
  (set `self.poleDirection` (- (`SceneComponent.RelativeLocation` (`self.pole_end`)) (`SceneComponent.K2_GetComponentLocation` (`self.pole`))))
  (bind _output_get (set `local.Aprime` (`KismetMathLibrary.MakeVector` _relativelocation_x _relativelocation_y _returnvalue_z)))
  (set `self.poleFloor` (- _output_get (`SceneComponent.K2_GetComponentLocation` (`self.pole`))))
  ;[1 1 1] u1 : pole direction, u2 : floor / cos(theta)=u1.u2/|u1||u2|
  (set `self.poleAngle` (/ (`KismetMathLibrary.Dot_VectorVector` (`self.poleDirection`) (`self.poleFloor`)) (* (`KismetMathLibrary.VSize` (`self.poleDirection`)) (`KismetMathLibrary.VSize` (`self.poleFloor`))))))

(fn `UserConstructionScript`)